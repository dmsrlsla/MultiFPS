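; Super-speed power-up, built on a parent power-up class, that makes the activating actor walk five times faster while active.
; On activation it stores that actor and multiplies the CharacterMovementComponent's current max speed into MaxWalkSpeed.
; On expiry it divides the current max speed by the same factor if the actor is still valid, without caching the original, then calls the parent to finish cleanup.
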(event EventBeginPlay)

(event Collision|EventActorBeginOverlap
  (params (OtherActor :type Actor%20Object%20Reference)))

(event EventTick
  (params (DeltaSeconds :type Float%20%28single-precision%29)))

(event EventOnActivated
  (params (ActiveFor :type Actor%20Object%20Reference))
  (bind _returnvalue (Actor|GetComponentbyClass ActiveFor "/Script/Engine.CharacterMovementComponent"))
  (Variables|Default|SetActiveForPlayer ActiveFor)
  (Variables|/Script/Engine.CharacterMovementComponent|SetMaxWalkSpeed _returnvalue (* (Class|MovementComponent|GetMaxSpeed _returnvalue) 5.0)) ; 이동 스피드 빨라짐.
)

(event EventOnPowerUpTicked)

(event EventOnExpired
  (bind _activeforplayer (Variables|Default|GetActiveForPlayer))
  (bind _returnvalue (Actor|GetComponentbyClass _activeforplayer "/Script/Engine.CharacterMovementComponent"))
  (Utilities|IsValid _activeforplayer
    (:Is%20Valid
      (Variables|/Script/Engine.CharacterMovementComponent|SetMaxWalkSpeed _returnvalue (/ (Class|MovementComponent|GetMaxSpeed _returnvalue) 5.0)) ; 파워업 종료시 이동속도 정상적으로 느려짐
    )
    (:Is%20Not%20Valid
      _))
  (|CallParentFunction) ; 부모 베이스에서 해당 액터 파괴
)

(fn ConstructionScript)